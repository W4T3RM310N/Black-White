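; BP_LoadLevel is a level-exit actor that fades each level in and loads the next one when its static mesh is overlapped.
; BeginPlay and overlap each create a BP_LoadLevelWidget, whose image opacity Tick animates to fade in or out.
; After a one-second delay, a hard-coded level-name chain opens the next level, advancing only from Level1 through Level4.
; Branches for Level5 through Level8, including return to MainMenu, are disconnected.
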(event `self.ReceiveBeginPlay`
  (bind _returnvalue (`|CreateWidget` "/Game/Blueprints/BP_LoadLevelWidget.BP_LoadLevelWidget_C"))
  (`UserWidget.AddToViewport` _returnvalue 0)
  (set `self.FadeIn` true)
  (`KismetSystemLibrary.Delay` 0.5)
  (set `self.bDoesTick` true)
  (`KismetSystemLibrary.Delay` 1.0)
  (`Widget.RemoveFromParent` _returnvalue)
  (set `self.TempTime` 0.0)
  (set `self.bDoesTick` false))

(event `self.ReceiveTick`
  (params (DeltaSeconds :type "Float (single-precision)"))
  (bind _temptime (`self.TempTime`))
  (if (`self.bDoesTick`)
    (if (`self.FadeIn`)
      (bind _output_get (set `self.TempTime` (+ _temptime DeltaSeconds)))
      (`Widget.SetRenderOpacity` (`/Game/Blueprints/BP_LoadLevelWidget.Image_98` (stale `self.ReceiveBeginPlay` _returnvalue)) (- 1.0 _output_get))
      (else
        (bind _output_get_2 (set `self.TempTime` (+ _temptime DeltaSeconds)))
        (`Widget.SetRenderOpacity` (`/Game/Blueprints/BP_LoadLevelWidget.Image_98` (stale `self.StaticMeshComponent.OnComponentBeginOverlap` _returnvalue)) _output_get_2)))))

(event `self.StaticMeshComponent.OnComponentBeginOverlap`
  (params (OverlappedComponent :type "PrimitiveComponent Object Reference") (OtherActor :type "Actor Object Reference") (OtherComp :type "PrimitiveComponent Object Reference") (OtherBodyIndex :type Integer) (bFromSweep :type Boolean) (SweepResult :type "HitResult Structure (by ref)"))
  (bind _returnvalue (`|CreateWidget` "/Game/Blueprints/BP_LoadLevelWidget.BP_LoadLevelWidget_C"))
  (`UserWidget.AddToViewport` _returnvalue 0)
  (set `self.FadeIn` false)
  (set `self.bDoesTick` true)
  (`KismetSystemLibrary.Delay` 1.0)
  (bind _returnvalue_2 (`GameplayStatics.GetCurrentLevelName` true))
  (if (`KismetStringLibrary.EqualEqual_StrStr` _returnvalue_2 "Level1")
    (`GameplayStatics.OpenLevel` "level2")
    (elif (`KismetStringLibrary.EqualEqual_StrStr` _returnvalue_2 "Level2")
      (`GameplayStatics.OpenLevel` "level3")
      (elif (`KismetStringLibrary.EqualEqual_StrStr` _returnvalue_2 "Level3")
        (`GameplayStatics.OpenLevel` "level4")
        (elif (`KismetStringLibrary.EqualEqual_StrStr` _returnvalue_2 "Level4")
          (`GameplayStatics.OpenLevel` "level5"))))))

(fn `UserConstructionScript`)