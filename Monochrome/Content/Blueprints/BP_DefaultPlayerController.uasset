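; Default player controller that opens the pause menu when the Pause input action is pressed.
; If no screen is shown, it creates and displays BP_PauseMenu, shows the cursor, switches to game-and-UI input focused on the menu and pauses the game.
; An IsScreenShown flag prevents duplicate menus; the logic to close the menu and unpause is present but unconnected, so it never runs here.
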(event `InputAction|Pause`
  (params (Key :type "Key Structure"))
  (:`Pressed`
    (if (not (`self.IsScreenShown`))
      (bind _returnvalue (`|CreateWidget` "/Game/Blueprints/BP_PauseMenu.BP_PauseMenu_C"))
      (`UserWidget.AddToViewport` _returnvalue 0)
      (bind _output_get (set `self.bShowMouseCursor` true))
      (`WidgetBlueprintLibrary.SetInputMode_GameAndUIEx` (`GameplayStatics.GetPlayerController` 0) _returnvalue "DoNotLock" _output_get)
      (set `self.IsScreenShown` true)
      (`GameplayStatics.SetGamePaused` true))))

(fn `UserConstructionScript`)